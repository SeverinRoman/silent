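; Player character Blueprint that handles movement, look, crouch and run through Enhanced Input, adding its mapping context on BeginPlay.
; Movement follows the control rotation, and crouch toggles on each press via a FlipFlop.
; Running is delegated to BPMoveComponent, starting on press and ending on release.
; A hard-wired F key turns on physics simulation for the mesh, with no way back.
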(event Input|EnhancedActionEvents|EnhancedInputActionIA_Move
  (params (ActionValue :type Vector%202D%20Structure) (ElapsedSeconds :type Float%20%28double-precision%29) (TriggeredSeconds :type Float%20%28double-precision%29) (InputAction :type Input%20Action%20Object%20Reference :default "/Game/AAASilent/Blueprint/Input/Actions/IA_Move.IA_Move"))
  (bind _returnvalue (Pawn|GetControlRotation :!class /Script/Engine.Pawn))
  (Pawn|Input|AddMovementInput (Math|Vector|GetForwardVector (Math|Rotator|MakeRotator 0.0 0.0 (.yaw (Pawn|GetControlRotation :!class /Script/Engine.Pawn)))) (.x ActionValue) false)
  (Pawn|Input|AddMovementInput (Math|Vector|GetRightVector (Math|Rotator|MakeRotator (.roll _returnvalue) 0.0 (.yaw _returnvalue))) (.y ActionValue) false))

(event Input|EnhancedActionEvents|EnhancedInputActionIA_Look
  (params (ActionValue :type Vector%202D%20Structure) (ElapsedSeconds :type Float%20%28double-precision%29) (TriggeredSeconds :type Float%20%28double-precision%29) (InputAction :type Input%20Action%20Object%20Reference :default "/Game/AAASilent/Blueprint/Input/Actions/IA_Look.IA_Look"))
  (Pawn|Input|AddControllerYawInput (.x ActionValue))
  (Pawn|Input|AddControllerPitchInput (.y ActionValue)))

(event Input|EnhancedActionEvents|EnhancedInputActionIA_Crouch
  (params (ActionValue :type Boolean) (ElapsedSeconds :type Float%20%28double-precision%29) (TriggeredSeconds :type Float%20%28double-precision%29) (InputAction :type Input%20Action%20Object%20Reference :default "/Game/AAASilent/Blueprint/Input/Actions/IA_Crouch.IA_Crouch"))
  (:Started
    (Utilities|FlowControl|FlipFlop
      (:A
        (Character|Crouch))
      (:B
        (Character|UnCrouch)))))

(event Input|EnhancedActionEvents|EnhancedInputActionIA_Run
  (params (ActionValue :type Boolean) (ElapsedSeconds :type Float%20%28double-precision%29) (TriggeredSeconds :type Float%20%28double-precision%29) (InputAction :type Input%20Action%20Object%20Reference :default "/Game/AAASilent/Blueprint/Input/Actions/IA_Run.IA_Run"))
  (bind _bp_movecomponent (Variables|Default|GetBP_MoveComponent))
  (bind _bp_movecomponent_2 (Variables|Default|GetBP_MoveComponent))
  (:Started
    (Utilities|IsValid _bp_movecomponent_2
      (:Is%20Valid
        (Default|Run _bp_movecomponent))))
  (:Completed
    (Utilities|IsValid _bp_movecomponent_2
      (:Is%20Valid
        (Default|UnRun _bp_movecomponent)))))

(event EventBeginPlay
  (Private|InitInput))

(event Input|KeyboardEvents|F
  (params (Key :type Key%20Structure :default "None"))
  (:Pressed
    (Physics|SetSimulatePhysics (Variables|Character|GetMesh) true)))

(fn ConstructionScript)

(fn InitInput
  (bind _asplayer_controller (Utilities|Casting|CastToPlayerController (Pawn|GetController)))
  (Input|AddMappingContext (PlayerController|LocalPlayerSubsystems|GetEnhancedInputLocalPlayerSubsystem _asplayer_controller) "/Game/AAASilent/Blueprint/Input/IMC_Input.IMC_Input" 0 "(bIgnoreAllPressedKeysUntilRelease=True,bForceImmediately=False,bNotifyUserSettings=False)"))