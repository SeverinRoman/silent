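; BP_Wind applies the UDW weather system's wind to a referenced Wind Directional Source when play begins.
; Init caches the source's component, then BeginPlay sets both its speed and strength from the same UDW wind intensity and rotates the actor along the UDW wind direction vector.
; The sync runs only once, so later wind changes are not followed.
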(event EventBeginPlay
  (Utilities|IsValid (Variables|Private|GetWindDirectionalSource)
    (:Is%20Valid
      (Private|Init)
      (Utilities|IsValid (Variables|Private|GetWindDirectionalSourceComponent)
        (:Is%20Valid
          (Class|WindDirectionalSourceComponent|SetSpeed (Variables|Private|GetWindDirectionalSourceComponent) (CallFunction|GetWindIntensity·𝖴𝖣𝖶))
          (Variables|/Script/Engine.WindDirectionalSourceComponent|SetStrength (Variables|Private|GetWindDirectionalSourceComponent) (CallFunction|GetWindIntensity·𝖴𝖣𝖶))
          (Transformation|SetActorRotation (Variables|Private|GetWindDirectionalSource) (Math|Conversions|RotationFromXVector (CallFunction|GetWindDirectionVector·𝖴𝖣𝖶))))))))

(fn ConstructionScript)

(fn Init
  (bind _winddirectionalsource (Variables|Private|GetWindDirectionalSource))
  (Utilities|IsValid _winddirectionalsource
    (:Is%20Valid
      (Variables|Private|SetWindDirectionalSourceComponent (Variables|/Script/Engine.WindDirectionalSource|GetComponent _winddirectionalsource))
      (return))))