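; BP_StateComponent is an actor component that tracks its owner's locomotion state: idle, move, crouch or falling.
; On begin play it caches the owner's CharacterMovementComponent, then each tick reads velocity, speed and facing-relative direction from it.
; Falling takes priority over crouching, which takes priority over a zero-speed idle/move check, and SetState calls CallStateChange only on changes.
; An optional debug flag prints these values on screen.
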(event EventBeginPlay
  (Private|Init))

(event EventTick
  (params (DeltaSeconds :type Float%20%28single-precision%29))
  (Private|UpdateData)
  (Private|UpdateState)
  (Private|Debug))

(fn GetState
  (return (Variables|Private|GetState)))

(fn SetState
  (params (NewState :type StateType%20Enum :default "NewEnumerator0"))
  (if (not (Utilities|Enum|Equal(Enum) NewState (Variables|Private|GetState)))
    (bind _output_get (Variables|Private|SetState NewState))
    (Default|CallStateChange _output_get)))

(fn Init
  (bind _returnvalue (Components|GetOwner))
  (Utilities|IsValid _returnvalue
    (:Is%20Valid
      (bind _output_get (Variables|Private|SetOwner _returnvalue))
      (Variables|Components|SetCharacterMovementComponent (Actor|GetComponentbyClass _output_get "/Script/Engine.CharacterMovementComponent")))))

(fn UpdateData
  (bind _charactermovementcomponent (Variables|Components|GetCharacterMovementComponent))
  (Utilities|IsValid (Variables|Private|GetOwner)
    (:Is%20Valid
      (Utilities|IsValid (Variables|Components|GetCharacterMovementComponent)
        (:Is%20Valid
          (Utilities|FlowControl|Sequence
            (:then_0
              (Utilities|IsValid _charactermovementcomponent
                (:Is%20Valid
                  (Variables|Private|SetVelocity (Variables|/Script/Engine.MovementComponent|GetVelocity _charactermovementcomponent))
                  (Variables|Private|SetSpeed (Math|Vector|VectorLength (Variables|Private|GetVelocity))))))
            (:then_1
              (Variables|Private|SetDirection (Class|KismetAnimationLibrary|CalculateDirection (Variables|Private|GetVelocity) (Transformation|GetActorRotation (Variables|Private|GetOwner)))))))))))

(fn Debug
  (if (Variables|Public|GetIsDebug)
    (Utilities|FlowControl|Sequence
      (:then_0
        (Development|PrintString (Utilities|String|Append (Utilities|String|ToString(Text) (Utilities|Text|ToText(String) "State: ")) (Utilities|String|EnumtoString (Variables|Private|GetState))) true true "(R=0.000000,G=0.660000,B=1.000000,A=1.000000)" 0.001))
      (:then_1
        (Development|PrintString (Utilities|String|Append (Utilities|String|ToString(Text) (Utilities|Text|ToText(String) "Velocity: ")) (Utilities|String|ToString(Vector) (Variables|Private|GetVelocity))) true true "(R=0.000000,G=0.660000,B=1.000000,A=1.000000)" 0.001))
      (:then_2
        (Development|PrintString (Utilities|String|Append (Utilities|String|ToString(Text) (Utilities|Text|ToText(String) "Direction: ")) (Utilities|String|ToString(Float) (Variables|Private|GetDirection))) true true "(R=0.000000,G=0.660000,B=1.000000,A=1.000000)" 0.001))
      (:then_3
        (Development|PrintString (Utilities|String|Append (Utilities|String|ToString(Text) (Utilities|Text|ToText(String) "Speed: ")) (Utilities|String|ToString(Float) (Variables|Private|GetSpeed))) true true "(R=0.000000,G=0.660000,B=1.000000,A=1.000000)" 0.001)))))

(fn UpdateState
  (Utilities|IsValid (Variables|Components|GetCharacterMovementComponent)
    (:Is%20Valid
      (if (AI|Components|NavMovement|IsFalling (Variables|Components|GetCharacterMovementComponent))
        (Public|SetState "NewEnumerator5")
        (elif (AI|Components|NavMovement|IsCrouching (Variables|Components|GetCharacterMovementComponent))
          (Public|SetState "NewEnumerator4")
          (else
            (switch Utilities|FlowControl|Switch|SwitchonStateType (Variables|Private|GetState)
              (:NewEnumerator1
                _)
              (:NewEnumerator2
                _)
              (:NewEnumerator4
                _)
              (:NewEnumerator5
                _))
            (if (== 0.0 (Variables|Private|GetSpeed))
              (Public|SetState "NewEnumerator1")
              (else
                (Public|SetState "NewEnumerator2")))))))))