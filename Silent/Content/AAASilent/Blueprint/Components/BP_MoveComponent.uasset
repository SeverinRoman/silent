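; BP_MoveComponent is an actor component that handles movement for its owning pawn or character: walking, running and crouching.
; On BeginPlay it caches the owner along with its movement, state and animation components.
; Move applies input relative to control rotation, while Run and UnRun switch max walk speed.
; Moving or crouching from STANDBY stops the current animation, and moving also sets the state to MOVE.
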(event EventBeginPlay
  (Private|Init))

(fn Run
  (Private|ChangeSpeed (Variables|Public|GetSpeedRun)))

(fn UnRun
  (Private|ChangeSpeed (Variables|Public|GetSpeedWalk)))

(fn Init
  (bind _returnvalue (Components|GetOwner))
  (Utilities|FlowControl|Sequence
    (:then_0
      (Utilities|IsValid _returnvalue
        (:Is%20Valid
          (Variables|Private|SetOwner _returnvalue)
          (bind _aspawn (Utilities|Casting|CastToPawn (Variables|Private|GetOwner)))
          (Variables|Private|SetPawn _aspawn)
          (bind _ascharacter (Utilities|Casting|CastToCharacter (Variables|Private|GetOwner)))
          (Variables|Private|SetCharacter _ascharacter))))
    (:then_1
      (Variables|Default|SetCharacterMovementComponent (Actor|GetComponentbyClass (Variables|Private|GetOwner) "/Script/Engine.CharacterMovementComponent"))
      (Variables|Default|SetStateComponent (Actor|GetComponentbyClass (Variables|Private|GetOwner) "/Game/AAASilent/Blueprint/Components/BP_StateComponent.BP_StateComponent_C"))
      (Variables|Default|SetAnimationComponent (Actor|GetComponentbyClass (Variables|Private|GetOwner) "/Game/AAASilent/Blueprint/Components/BP_AnimationComponent.BP_AnimationComponent_C")))))

(fn ChangeSpeed
  (params (NewSpeed :type Float%20%28double-precision%29))
  (bind _charactermovementcomponent (Variables|Default|GetCharacterMovementComponent))
  (Utilities|IsValid _charactermovementcomponent
    (:Is%20Valid
      (Variables|/Script/Engine.CharacterMovementComponent|SetMaxWalkSpeed _charactermovementcomponent NewSpeed))))

(fn Move
  (params (X :type Float%20%28double-precision%29) (Y :type Float%20%28double-precision%29))
  (bind _pawn (Variables|Private|GetPawn))
  (bind _returnvalue (Pawn|GetControlRotation _pawn :!class /Script/Engine.Pawn))
  (Utilities|IsValid (Variables|Private|GetPawn)
    (:Is%20Valid
      (Pawn|Input|AddMovementInput (Variables|Private|GetPawn) (Math|Vector|GetForwardVector (Math|Rotator|MakeRotator 0.0 0.0 (.yaw (Pawn|GetControlRotation (Variables|Private|GetPawn) :!class /Script/Engine.Pawn)))) X false)
      (Pawn|Input|AddMovementInput (Variables|Private|GetPawn) (Math|Vector|GetRightVector (Math|Rotator|MakeRotator (.roll _returnvalue) 0.0 (.yaw _returnvalue))) Y false)
      (Private|CheckStandby))))

(fn Crouch
  (Utilities|IsValid (Variables|Private|GetCharacter)
    (:Is%20Valid
      (Utilities|IsValid (Variables|Default|GetAnimationComponent)
        (:Is%20Valid
          (Utilities|IsValid (Variables|Default|GetStateComponent)
            (:Is%20Valid
              (bind _state (Default|GetState (Variables|Default|GetStateComponent)))
              (switch Utilities|FlowControl|Switch|SwitchonStateType _state
                (:NewEnumerator1
                  (Character|Crouch (Variables|Private|GetCharacter) :!label _label))
                (:NewEnumerator2
                  (goto _label))
                (:NewEnumerator7
                  (Default|Stop (Variables|Default|GetAnimationComponent))
                  (Character|Crouch (Variables|Private|GetCharacter)))))))))))

(fn UnCrouch
  (Utilities|IsValid (Variables|Private|GetCharacter)
    (:Is%20Valid
      (Character|UnCrouch (Variables|Private|GetCharacter)))))

(fn CheckStandby
  (Utilities|IsValid (Variables|Default|GetAnimationComponent)
    (:Is%20Valid
      (Utilities|IsValid (Variables|Default|GetStateComponent)
        (:Is%20Valid
          (bind _state (Default|GetState (Variables|Default|GetStateComponent)))
          (if (Utilities|Enum|Equal(Enum) _state "NewEnumerator7")
            (Default|Stop (Variables|Default|GetAnimationComponent))
            (Default|SetState (Variables|Default|GetStateComponent) "NewEnumerator2")))))))