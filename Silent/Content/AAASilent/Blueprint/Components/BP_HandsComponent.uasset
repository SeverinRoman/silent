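; Hands component that finds blocking surfaces beside its owner and exposes hit flags and locations for left and right hands.
; Each tick it line-traces from a height offset: left, right, and right-forward diagonal at shorter range.
; The right side hit takes priority over the diagonal, which has its own flag.
; Each hand keeps its last hit location when traces miss, and a debug flag draws the traces.
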(event EventBeginPlay
  (Private|Init))

(event EventTick
  (params (DeltaSeconds :type Float%20%28single-precision%29))
  (Utilities|IsValid (Variables|Private|GetOwner)
    (:Is%20Valid
      (Utilities|FlowControl|Sequence
        (:then_0
          (Private|TraceRightHand))
        (:then_1
          (Private|TraceLeftHand))))))

(fn Init
  (bind _returnvalue (Components|GetOwner))
  (Utilities|IsValid _returnvalue
    (:Is%20Valid
      (Variables|Private|SetOwner _returnvalue)
      (if (Variables|Public|GetIsDebug)
        (Variables|Private|SetDebugType 1)
        (else
          (Variables|Private|SetDebugType 0))))))

(fn Trace
  (params (Direction :type Vector) (Height :type Float%20%28double-precision%29) (Distance :type Float%20%28double-precision%29))
  (bind _returnvalue (* Direction Distance))
  (bind _owner (Variables|Private|GetOwner))
  (bind _returnvalue_2 (Transformation|GetActorLocation _owner))
  (bind (_x _y _z) (Math|Vector|BreakVector _returnvalue_2))
  (bind _returnvalue_3 (+ _returnvalue_2 _returnvalue))
  (LocalVariables|SetHeigh Height)
  (bind _outhit (Class|KismetSystemLibrary|LineTraceSinglebyProfile (Math|Vector|MakeVector _x _y (+ _z (LocalVariables|GetHeigh))) (Math|Vector|MakeVector (.x _returnvalue_3) (.y _returnvalue_3) (+ (.z _returnvalue_3) (LocalVariables|GetHeigh))) "BlockAll" false 0 (Utilities|Enum|ByteToEnumEDrawDebugTrace (Variables|Private|GetDebugType)) true))
  (return (.bBlockingHit (Collision|BreakHitResult _outhit)) (.Location (Collision|BreakHitResult _outhit))))

(fn TraceLeftHand
  (bind (_ishit _location) (Private|Trace (* (Transformation|GetActorRightVector (Variables|Private|GetOwner)) -1.0) (Variables|Public|GetHeigh) (Variables|public|GetDistance)))
  (bind _output_get (Variables|Private|SetIsHitLeftHand _ishit))
  (if _output_get
    (bind _output_get_2 (Variables|Private|SetLeftHandLocation _location))
    (Variables|Private|SetBufferLeft _output_get_2)
    (else
      (Variables|Private|SetLeftHandLocation (Variables|Private|GetBufferLeft)))))

(fn TraceRightHand
  (bind _owner (Variables|Private|GetOwner))
  (Utilities|FlowControl|Sequence
    (:then_0
      (bind (_ishit _location) (Private|Trace (Transformation|GetActorRightVector (Variables|Private|GetOwner)) (Variables|Public|GetHeigh) (Variables|public|GetDistance)))
      (bind _output_get (LocalVariables|SetIsHitRight _ishit))
      (if _output_get
        (LocalVariables|SetRightLocation _location)))
    (:then_1
      (bind (_ishit_2 _location_2) (Private|Trace (+ (Transformation|GetActorForwardVector _owner) (Transformation|GetActorRightVector _owner)) (Variables|Public|GetHeigh) (/ (Variables|public|GetDistance) 1.5)))
      (bind _output_get_2 (LocalVariables|SetIsHitForward _ishit_2))
      (if _output_get_2
        (LocalVariables|SetForwardLocation _location_2)))
    (:then_2
      (if (LocalVariables|GetIsHitRight)
        (Variables|Private|SetIsHitRightHand true)
        (Variables|Private|SetRightHandLocation (LocalVariables|GetRightLocation))
        (Variables|Private|SetBufferRight (LocalVariables|GetRightLocation))
        (Variables|Private|SetIsHitRightHandForward false)
        (elif (LocalVariables|GetIsHitForward)
          (Variables|Private|SetIsHitRightHandForward true)
          (Variables|Private|SetRightHandLocation (LocalVariables|GetForwardLocation))
          (Variables|Private|SetBufferRight (LocalVariables|GetForwardLocation))
          (LocalVariables|SetIsHitRight false)
          (else
            (Variables|Private|SetIsHitRightHandForward false)
            (Variables|Private|SetIsHitRightHand false)
            (Variables|Private|SetRightHandLocation (Variables|Private|GetBufferRight))))))))

(fn GetLeftHandLocation
  (return (Variables|Private|GetLeftHandLocation)))

(fn GetRightHandLocation
  (return (Variables|Private|GetRightHandLocation)))

(fn GetIsHitLeftHand
  (return (Variables|Private|GetIsHitLeftHand)))

(fn GetIsHitRightHand
  (return (Variables|Private|GetIsHitRightHand)))

(fn GetIsHitRightHandForward
  (return (Variables|Private|GetIsHitRightHandForward)))