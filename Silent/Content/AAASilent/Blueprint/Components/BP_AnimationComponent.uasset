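; Actor component that plays animation montages on its owner's skeletal mesh by looking up a key in an Animations map.
; On BeginPlay, Init caches the owner, its SkeletalMeshComponent and that mesh's AnimInstance.
; AnimationStart plays the matching montage through PlayMontage and calls AnimationEnd on completion only, with no handling for interruption or missing keys.
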(event Custom|AnimationStart
  (params (Animation :type AnimationType%20Enum :default "NewEnumerator0"))
  (Utilities|IsValid (Variables|Default|GetSkeletalMesh)
    (:Is%20Valid
      (if (Utilities|Map|Contains (Variables|Public|GetAnimations) Animation)
        (Animation|Montage|PlayMontage (Variables|Default|GetSkeletalMesh) (.Value (Utilities|Map|Find (Variables|Public|GetAnimations) Animation))
          (:OnCompleted
            (Default|CallAnimationEnd)))))))

(event EventBeginPlay
  (Private|Init))

(fn Init
  (bind _returnvalue (Components|GetOwner))
  (Utilities|IsValid _returnvalue
    (:Is%20Valid
      (bind _output_get (Variables|Private|SetOwner _returnvalue))
      (Utilities|IsValid (Actor|GetComponentbyClass _output_get "/Script/Engine.SkeletalMeshComponent")
        (:Is%20Valid
          (Variables|Default|SetSkeletalMesh (Actor|GetComponentbyClass _output_get "/Script/Engine.SkeletalMeshComponent"))
          (Utilities|IsValid (Components|SkeletalMesh|GetAnimInstance (Actor|GetComponentbyClass _output_get "/Script/Engine.SkeletalMeshComponent"))
            (:Is%20Valid
              (Variables|Components|SetAnimInstance (Components|SkeletalMesh|GetAnimInstance (Actor|GetComponentbyClass _output_get "/Script/Engine.SkeletalMeshComponent"))))))))))