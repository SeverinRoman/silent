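; BP_StandbyComponent is an actor component that plays random standby animations when its owner stays idle.
; At BeginPlay it finds the owner's state and animation components.
; A retriggerable delay restarts on changes to IDLE or STANDBY; if still IDLE when it expires, it starts a random animation and sets STANDBY.
; The animation-end callback returns the state to IDLE, so the cycle repeats.
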(event Custom|CustomEvent
  (params (StateType :type EStateType%20Enum :default "NONE"))
  (bind _animationcomponent (Variables|Default|GetAnimationComponent))
  (switch Utilities|FlowControl|Switch|SwitchonEStateType StateType
    (:IDLE
      _)
    (:STANDBY
      _))
  (Utilities|FlowControl|RetriggerableDelay (Variables|Public|GetDelay) :!label _label)
  (if (Utilities|Enum|Equal(Enum) (Default|GetState (Variables|Default|GetStateComponent)) "IDLE")
    (Default|AnimationStart _animationcomponent (.OutItem (Utilities|Array|Random (Variables|Public|GetAnimations))))
    (EventDispatchers|BindEventtoAnimationEnd _animationcomponent (delegate Custom|OnAnimationEnd))
    (Default|SetState (Variables|Default|GetStateComponent) "STANDBY")
    (goto _label)))

(event Custom|OnAnimationEnd
  (Default|SetState (Variables|Default|GetStateComponent) "IDLE"))

(event EventBeginPlay
  (bind _animationcomponent (Variables|Default|GetAnimationComponent))
  (Private|Init)
  (Utilities|IsValid (Variables|Default|GetStateComponent)
    (:Is%20Valid
      (Utilities|IsValid (Variables|Default|GetAnimationComponent)
        (:Is%20Valid
          (EventDispatchers|BindEventtoOnStateChange (Variables|Default|GetStateComponent) (delegate Custom|CustomEvent))
          (Utilities|FlowControl|RetriggerableDelay (Variables|Public|GetDelay) :!label _label)
          (if (Utilities|Enum|Equal(Enum) (Default|GetState (Variables|Default|GetStateComponent)) "IDLE")
            (Default|AnimationStart _animationcomponent (.OutItem (Utilities|Array|Random (Variables|Public|GetAnimations))))
            (EventDispatchers|BindEventtoAnimationEnd _animationcomponent (delegate Custom|OnAnimationEnd))
            (Default|SetState (Variables|Default|GetStateComponent) "STANDBY")
            (goto _label)))))))

(fn Init
  (bind _returnvalue (Components|GetOwner))
  (Utilities|IsValid _returnvalue
    (:Is%20Valid
      (Variables|Components|SetOwner _returnvalue)
      (Utilities|IsValid (Actor|GetComponentbyClass (Variables|Components|GetOwner) "/Game/AAASilent/Blueprint/Components/BP_StateComponent.BP_StateComponent_C")
        (:Is%20Valid
          (Variables|Default|SetStateComponent (Actor|GetComponentbyClass (Variables|Components|GetOwner) "/Game/AAASilent/Blueprint/Components/BP_StateComponent.BP_StateComponent_C"))
          (Utilities|IsValid (Actor|GetComponentbyClass (Variables|Components|GetOwner) "/Game/AAASilent/Blueprint/Components/BP_AnimationComponent.BP_AnimationComponent_C")
            (:Is%20Valid
              (Variables|Default|SetAnimationComponent (Actor|GetComponentbyClass (Variables|Components|GetOwner) "/Game/AAASilent/Blueprint/Components/BP_AnimationComponent.BP_AnimationComponent_C")))))))))