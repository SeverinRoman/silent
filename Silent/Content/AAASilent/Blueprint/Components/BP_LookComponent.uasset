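; BP_LookComponent is an actor component that tracks a point in the world where its owner's camera is looking.
; On BeginPlay it caches the owner and the owner's CameraComponent.
; Each Tick it sets LookLocation to a fixed distance along the camera's forward vector, with no trace, so obstacles do not affect the point.
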(event EventBeginPlay
  (Private|Init))

(event EventTick
  (params (DeltaSeconds :type Float%20%28single-precision%29))
  (Private|Look))

(fn Init
  (bind _returnvalue (Components|GetOwner))
  (Utilities|IsValid _returnvalue
    (:Is%20Valid
      (Variables|Public|SetOwner _returnvalue)
      (Variables|Default|SetCameraComponent (Actor|GetComponentbyClass (Variables|Public|GetOwner) "/Script/Engine.CameraComponent")))))

(fn Look
  (bind _cameracomponent (Variables|Default|GetCameraComponent))
  (Utilities|IsValid (Variables|Default|GetCameraComponent)
    (:Is%20Valid
      (Variables|Public|SetLookLocation (+ (Transformation|GetWorldLocation _cameracomponent) (* (Math|Vector|GetForwardVector _cameracomponent) 1e+03))))))